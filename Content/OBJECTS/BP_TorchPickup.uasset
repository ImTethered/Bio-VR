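; BP_TorchPickup is a pickup actor that gives the player a torch when used.
; On the OnUsed event it destroys itself, then casts the first player character to FirstPersonCharacter and sets HasTorch to true.
; BeginPlay, overlap and Tick are disabled stubs, and the construction script only calls its parent.
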(event `self.On Used`
  (params (character :type "Character Object Reference"))
  (`self.K2_DestroyActor`)
  (bind _asfirst_person_character (cast `/Game/CONTENT/FirstPersonBP/Blueprints/FirstPersonCharacter` (`GameplayStatics.GetPlayerCharacter` 0)))
  (set `/Game/CONTENT/FirstPersonBP/Blueprints/FirstPersonCharacter.hasTorch` true _asfirst_person_character))

(fn `UserConstructionScript`
  (`parent.UserConstructionScript`))