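; Teleporter trigger that sends the VR player pawn to a fixed location and advances a level counter.
; On overlap it fades the camera out, waits, casts to VR_PlayerPawn, teleports, then fades back in.
; A switch on the counter spawns torch pickups and level doors or destroys indexed MagicDoor actors, with nothing for level 3.
; Fade-out precedes the pawn cast, and the enemy-spawn logic is unconnected.
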(event `self.ReceiveBeginPlay`
  (`KismetSystemLibrary.PrintString` (`KismetStringLibrary.Conv_IntToString` (`self.Current_Level`))))

(event `self.ReceiveActorBeginOverlap`
  (params (OtherActor :type "Actor Object Reference"))
  (bind _returnvalue (`KismetMathLibrary.MakeColor` 0.0))
  (bind _fade_out_duration (`self.Fade Out Duration`))
  (`PlayerCameraManager.StartCameraFade` (`GameplayStatics.GetPlayerCameraManager` 0) 0.0 1.0 _fade_out_duration _returnvalue false true)
  (`KismetSystemLibrary.Delay` _fade_out_duration)
  (bind _asvr_player_pawn (cast `/Game/VR_PLAYER/VR_PlayerPawn` OtherActor))
  (`self.K2_TeleportTo` :`self` _asvr_player_pawn :`DestLocation` (4138.0 1433.0 620.0))
  (`PlayerCameraManager.StartCameraFade` (`GameplayStatics.GetPlayerCameraManager` 0) 1.0 0.0 _fade_out_duration _returnvalue false false)
  (bind _result (`/Engine/EditorBlueprintResources/StandardMacros.IncrementInt` (`self.Current_Level`))
    (:`  `
      (bind _output_get (set `self.Current_Level` _result))
      (`KismetSystemLibrary.PrintString` (`KismetStringLibrary.Conv_IntToString` _output_get))
      (switch `int` _output_get
        (:`1`
          (`|SpawnActorFromClass` "/Game/OBJECTS/BP_TorchPickup.BP_TorchPickup_C" (`KismetMathLibrary.Conv_VectorToTransform` (2810.0 3983.0 590.0)) "AlwaysSpawn" "OverrideRootScale" null null)
          (`|SpawnActorFromClass` "/Game/OBJECTS/LevelDoor.LevelDoor_C" (`KismetMathLibrary.Conv_VectorToTransform` (2840.0 5855.422363 500.0)) "AlwaysSpawn" "OverrideRootScale" null null))
        (:`2`
          (bind _asmagic_door (castclass `/Game/OBJECTS/MagicDoor` "/Game/OBJECTS/MagicDoor.MagicDoor_C"))
          (bind _outactors (`GameplayStatics.GetAllActorsOfClass` _asmagic_door))
          (`self.K2_DestroyActor` (`|GetArrayItem` _outactors 2))
          (`|SpawnActorFromClass` "/Game/OBJECTS/BP_TorchPickup.BP_TorchPickup_C" (`KismetMathLibrary.Conv_VectorToTransform` (1970.0 3750.0 600.0)) "AlwaysSpawn" "OverrideRootScale" null null)
          (`|SpawnActorFromClass` "/Game/OBJECTS/LevelDoor1.LevelDoor1_C" (`KismetMathLibrary.Conv_VectorToTransform` (2840.0 5855.422363 500.0)) "AlwaysSpawn" "OverrideRootScale" null null))
        (:`4`
          (bind _asmagic_door_2 (castclass `/Game/OBJECTS/MagicDoor` "/Game/OBJECTS/MagicDoor.MagicDoor_C"))
          (bind _outactors_2 (`GameplayStatics.GetAllActorsOfClass` _asmagic_door_2))
          (`self.K2_DestroyActor` (`|GetArrayItem` _outactors_2 1))
          (`|SpawnActorFromClass` "/Game/OBJECTS/BP_TorchPickup.BP_TorchPickup_C" (`KismetMathLibrary.Conv_VectorToTransform` (3481.081543 2696.022217 582.271606)) "AlwaysSpawn" "OverrideRootScale" null null)
          (`|SpawnActorFromClass` "/Game/OBJECTS/LevelDoor2.LevelDoor2_C" (`KismetMathLibrary.Conv_VectorToTransform` (2840.0 5855.422363 500.0)) "AlwaysSpawn" "OverrideRootScale" null null))
        (:`5`
          (`|SpawnActorFromClass` "/Game/OBJECTS/BP_TorchPickup.BP_TorchPickup_C" (`KismetMathLibrary.Conv_VectorToTransform` (2810.0 3983.0 590.0)) "AlwaysSpawn" "OverrideRootScale" null null)
          (`|SpawnActorFromClass` "/Game/OBJECTS/LevelDoor3.LevelDoor3_C" (`KismetMathLibrary.Conv_VectorToTransform` (2840.0 5855.422363 500.0)) "AlwaysSpawn" "OverrideRootScale" null null))
        (:`6`
          (bind _asmagic_door_3 (castclass `/Game/OBJECTS/MagicDoor` "/Game/OBJECTS/MagicDoor.MagicDoor_C"))
          (bind _outactors_3 (`GameplayStatics.GetAllActorsOfClass` _asmagic_door_3))
          (`self.K2_DestroyActor` (`|GetArrayItem` _outactors_3)))))))

(event `self.ReceiveActorEndOverlap`
  (params (OtherActor :type "Actor Object Reference")))

(fn `UserConstructionScript`)